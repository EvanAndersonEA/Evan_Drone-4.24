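; BP_Pathfinder is a drone-game actor that lays out an arched trail of gates toward an XMark at BeginPlay.
; It moves the last point of its three-point spline to the XMark, then centers the middle point along the path, raised above the start.
; It spawns twenty Gate actors at even distances along the curve, using world-space positions and the spline's local-space rotation.
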(event `self.ReceiveBeginPlay`
  (bind (_returnvalue_x _returnvalue_y _returnvalue_z) (`KismetMathLibrary.BreakVector` (`SplineComponent.GetLocationAtSplinePoint` (`self.Spline`) 0 "Local")))
  (bind (_returnvalue_x_2 _returnvalue_y_2) (`KismetMathLibrary.BreakVector` (`SplineComponent.GetLocationAtDistanceAlongSpline` (`self.Spline`) (/ (`SplineComponent.GetDistanceAlongSplineAtSplinePoint` (`self.Spline`) 2) 2.0) "Local")))
  (`SplineComponent.SetLocationAtSplinePoint` (`self.Spline`) 2 (`self.K2_GetActorLocation` (`self.XMark`)) "World" true)
  (`SplineComponent.SetLocationAtSplinePoint` (`self.Spline`) 1 (`KismetMathLibrary.MakeVector` _returnvalue_x_2 _returnvalue_y_2 (+ _returnvalue_z 500.0)) "Local" true)
  (for _index (range 1 21)
    (bind _returnvalue (* (`SplineComponent.GetDistanceAlongSplineAtSplinePoint` (`self.Spline`) 2) (* (`KismetMathLibrary.Conv_IntToDouble` _index) 0.05)))
    (`|SpawnActorFromClass` "/Game/Drone/Actors/Gate.Gate_C" (`KismetMathLibrary.MakeTransform` (`SplineComponent.GetLocationAtDistanceAlongSpline` (`self.Spline`) _returnvalue "World") (`SplineComponent.GetRotationAtDistanceAlongSpline` (`self.Spline`) _returnvalue "Local")) "Undefined" "OverrideRootScale" null null)))

(fn `UserConstructionScript`)